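; BP_Player is the player Blueprint, with key bindings that appear to exercise enemy AI states and senses.
; Key 1 alternates the AI controller of an enemy found by class between attacking the player and passive.
; F makes a noise with an explosion effect and sound at the player's location.
; X reports a damage event on an enemy to AI perception, with the player as instigator.
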(event `Key|One`
  (params (Key :type "Key Structure"))
  (:`Pressed`
    (bind _returnvalue (`GameplayStatics.GetActorOfClass` "/Game/LegacyHunter/Enemy/BP_Enemy_Base.BP_Enemy_Base_C"))
    (bind _asbp_aic_enemy_base (cast `/Game/LegacyHunter/Enemy/AI/BP_AIC_Enemy_Base` (`AIBlueprintHelperLibrary.GetAIController` _returnvalue)))
    (`/Engine/EditorBlueprintResources/StandardMacros.FlipFlop`
      (:`A`
        (`/Game/LegacyHunter/Enemy/AI/BP_AIC_Enemy_Base.SetStateAsAttacking` _asbp_aic_enemy_base self))
      (:`B`
        (`/Game/LegacyHunter/Enemy/AI/BP_AIC_Enemy_Base.SetStateAsPassive` _asbp_aic_enemy_base)))))

(event `Key|F`
  (params (Key :type "Key Structure"))
  (bind _returnvalue (`self.K2_GetActorLocation`))
  (:`Pressed`
    (`self.MakeNoise` 1.0 self _returnvalue)
    (`GameplayStatics.SpawnEmitterAtLocation` "/Game/StarterContent/Particles/P_Explosion.P_Explosion" _returnvalue)
    (`GameplayStatics.PlaySoundAtLocation` "/Game/StarterContent/Audio/Explosion01.Explosion01" _returnvalue (struct) 1.0 1.0 0.0 null null null null)))

(event `Key|X`
  (params (Key :type "Key Structure"))
  (:`Pressed`
    (bind _returnvalue (`GameplayStatics.GetActorOfClass` "/Game/LegacyHunter/Enemy/BP_Enemy_Base.BP_Enemy_Base_C"))
    (`AISense_Damage.ReportDamageEvent` _returnvalue self 10.0 (`self.K2_GetActorLocation`))))

(fn `UserConstructionScript`)