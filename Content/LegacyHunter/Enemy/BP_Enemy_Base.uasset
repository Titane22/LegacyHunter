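; Base enemy character for LegacyHunter that spawns a sword on BeginPlay and attaches it to its right-hand socket.
; Attack plays a sword-slash montage and fires the OnAttackEnd dispatcher whether the montage completes or is interrupted.
; Helper functions supply attack and defend radii and a patrol route, and map a speed state from idle to sprinting onto the character's max walk speed.
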(event `self.ReceiveBeginPlay`
  (`self.WieldSword`))

(event `Attack`
  (`|PlayMontage` (`self.Mesh`) "/Game/LegacyHunter/Animations/Character/MONT_sword-slash.MONT_sword-slash"
    (:`OnCompleted`
      _)
    (:`OnInterrupted`
      _))
  (`self.OnAttackEnd`))

(event `WieldSword`
  (bind _returnvalue (`|SpawnActorFromClass` "/Game/Weapons/BT_Sword.BT_Sword_C" (`self.GetTransform`) "Undefined" "MultiplyWithRoot" null null))
  (`self.K2_AttachToComponent` _returnvalue (`self.Mesh`) "hand_r_sword_socket" "SnapToTarget" "SnapToTarget" "SnapToTarget" true)
  (set `self.IsWieldingSword` true))

(fn `GetIdealRange`
  (returns (AttackRadius :type "Float (double-precision)") (DefendRadius :type "Float (double-precision)"))
  (return 150.0 350.0))

(fn `GetPatrolRoute`
  (returns (PatrolRoute :type "/Game/LegacyHunter/Enemy/AI/BP_PatrolRoute Object Reference"))
  (return (`self.PatrolRoute`)))

(fn `SetMovementSpeed`
  (params (Speed :type "/Game/LegacyHunter/Enemy/AI/Enums/E_MovementSpeed Enum" :default "NewEnumerator0"))
  (returns (SpeedValue :type "Float (double-precision)"))
  (set `CharacterMovementComponent.MaxWalkSpeed` (select `/Game/LegacyHunter/Enemy/AI/Enums/E_MovementSpeed` Speed :`NewEnumerator1` 100.0 :`NewEnumerator2` 300.0 :`NewEnumerator3` 500.0 :!type "Float (single-precision)") (`self.CharacterMovement`))
  (return 0.0))

(fn `UserConstructionScript`)